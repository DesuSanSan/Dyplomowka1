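; NPC actor that talks to the player and then opens a shop.
; Interface overlap events switch the character's ActionEnum, and each Talk call advances TalkIndex through the Dialogue array in a Dialogue_W widget.
; Past the second line, it shows a random later line briefly while opening Shop_W, blending the camera to itself, showing the cursor and hiding the player.
; Z calls XD on ShopUI.
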(event OnComponentBeginOverlap(Interface)
  (params (OverlappedComponent :type Primitive%20Component%20Object%20Reference) (OtherActor :type Actor%20Object%20Reference) (OtherComp :type Primitive%20Component%20Object%20Reference) (OtherBodyIndex :type Integer) (bFromSweep :type Boolean) (SweepResult :type Hit%20Result%20Structure%20%28by%20ref%29))
  (Variables|/Game/ThirdPerson/Blueprints/BP_ThirdPersonCharacter.BP_ThirdPersonCharacter_C|SetActionEnum (Variables|Default|GetCharRef) "NewEnumerator0"))

(event OnComponentEndOverlap(Interface)
  (params (OverlappedComponent :type Primitive%20Component%20Object%20Reference) (OtherActor :type Actor%20Object%20Reference) (OtherComp :type Primitive%20Component%20Object%20Reference) (OtherBodyIndex :type Integer))
  (Variables|/Game/ThirdPerson/Blueprints/BP_ThirdPersonCharacter.BP_ThirdPersonCharacter_C|SetActionEnum (Variables|Default|GetCharRef) "NewEnumerator3"))

(event EventBeginPlay
  (bind _returnvalue (Actor|GetActorOfClass "/Game/ThirdPerson/Blueprints/BP_ThirdPersonCharacter.BP_ThirdPersonCharacter_C"))
  (Variables|Default|SetCharRef _returnvalue))

(event EventTalk
  (Math|Integer|IncrementInt (Variables|Default|GetTalkIndex)
    (:%20%20
      (if (> (Variables|Default|GetTalkIndex) 2)
        (if (not (Variables|Default|GetShopIsOn))
          (Variables|Default|SetTalkIndex (Math|Random|RandomIntegerinRange 3 5))
          (Game|Player|SetViewTargetwithBlend (Game|GetPlayerController 0) self 0.2 "VTBlend_Linear" 0.0 false)
          (bind _returnvalue (UserInterface|CreateWidget "/Game/Widgets/Shop_W.Shop_W_C" 0 self))
          (UserInterface|Viewport|AddtoViewport _returnvalue 0)
          (Variables|/Script/Engine.PlayerController|SetbShowMouseCursor (Game|GetPlayerController 0) true)
          (Rendering|SetActorHiddenInGame (Game|GetPlayerCharacter 0) true)
          (if (Variables|Default|GetDialogueUIOn)
            _
            (else
              (bind _returnvalue_2 (UserInterface|CreateWidget "/Game/ThirdPerson/Blueprints/Dialogue_W.Dialogue_W_C" (Game|GetPlayerController 0)))
              (bind _output_get (Variables|Default|SetUI _returnvalue_2))
              (UserInterface|Viewport|AddtoViewport _output_get 0)
              (Variables|Default|SetDialogueUIOn true)))
          (Rendering|Components|TextRender|SetText (Variables|/Game/ThirdPerson/Blueprints/Dialogue_W.Dialogue_W_C|GetTalkText (Variables|Default|GetUI)) (Utilities|Text|ToText(String) (Utilities|Array|Get(acopy) (Variables|Default|GetDialogue) (Variables|Default|GetTalkIndex))))
          (Variables|Default|SetShopIsOn true)
          (bind _asbp_third_person_character (Utilities|Casting|CastToBP_ThirdPersonCharacter (Game|GetPlayerCharacter 0)))
          (Variables|/Game/ThirdPerson/Blueprints/BP_ThirdPersonCharacter.BP_ThirdPersonCharacter_C|SetDoingAction _asbp_third_person_character true)
          (Utilities|FlowControl|Delay 1.0)
          (Variables|Default|SetDialogueIsOn false)
          (Widget|RemovefromParent (Variables|Default|GetUI))
          (Variables|Default|SetDialogueUIOn false))
        (elif (or (< (Variables|Default|GetTalkIndex) (Utilities|Array|Length (Variables|Default|GetDialogue))) (Variables|Default|GetDialogueIsOn))
          (if (Variables|Default|GetDialogueUIOn)
            _
            (else
              (bind _returnvalue_3 (UserInterface|CreateWidget "/Game/ThirdPerson/Blueprints/Dialogue_W.Dialogue_W_C" (Game|GetPlayerController 0)))
              (bind _output_get_2 (Variables|Default|SetUI _returnvalue_3))
              (UserInterface|Viewport|AddtoViewport _output_get_2 0)
              (Variables|Default|SetDialogueUIOn true)))
          (Rendering|Components|TextRender|SetText (Variables|/Game/ThirdPerson/Blueprints/Dialogue_W.Dialogue_W_C|GetTalkText (Variables|Default|GetUI)) (Utilities|Text|ToText(String) (Utilities|Array|Get(acopy) (Variables|Default|GetDialogue) (Variables|Default|GetTalkIndex))))
          (Utilities|FlowControl|Delay 2.0)
          (Variables|Default|SetDialogueUIOn true)
          (else
            (Variables|Default|SetDialogueIsOn false)
            (Widget|RemovefromParent (Variables|Default|GetUI))))))))

(event Input|KeyboardEvents|Z
  (params (Key :type Key%20Structure :default "None"))
  (:Pressed
    (Default|XD (Variables|Default|GetShopUI))))

(fn ConstructionScript)